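; BP_PlatformEnemy is a platformer enemy that reverses at ledges and dies when the player bounces on it.
; When its LedgeDetection component ends an overlap, it calls TurnCharacter to face the other direction.
; The PlayerBouncedonEnemy event destroys the actor, while BeginPlay, overlap and Tick are disabled stubs.
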(event OnComponentEndOverlap(LedgeDetection)
  (params (OverlappedComponent :type Primitive%20Component%20Object%20Reference) (OtherActor :type Actor%20Object%20Reference) (OtherComp :type Primitive%20Component%20Object%20Reference) (OtherBodyIndex :type Integer))
  ;[1 1 1] When the ledge detection ends overlap, turn the enemy toward the other direction
  (CallFunction|TurnCharacter))

(event EventBeginPlay
  (|CallParentFunction) ; This node is disabled and will not be called.\nDrag off pins to build functionality.
)

(event Collision|EventActorBeginOverlap
  (params (OtherActor :type Actor%20Object%20Reference))
  (|CallParentFunction OtherActor) ; This node is disabled and will not be called.\nDrag off pins to build functionality.
)

(event EventTick
  (params (DeltaSeconds :type Float%20%28single-precision%29))
  (|CallParentFunction DeltaSeconds) ; This node is disabled and will not be called.\nDrag off pins to build functionality.
)

(event EventPlayerBouncedonEnemy
  (Actor|DestroyActor))

(fn ConstructionScript
  (|CallParentFunction))