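; Player character Blueprint for a platformer, handling X-axis movement, bouncing, pushing boxes, pause input, and damage with respawn.
; An overlap trigger launches the falling player off actors implementing BPI_PlayerBounceInterface, while MushroomBounce reflects and amplifies downward velocity.
; Damage freezes the player through the PlayerSM state, then calls OnPlayerDeath and respawns after a delay.
; Jump, fall, launch and landing events drive animation node jumps, sounds or airborne wind audio.
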(event OnComponentBeginOverlap(PlayerBounceDetection)
  (params (OverlappedComponent :type Primitive%20Component%20Object%20Reference) (OtherActor :type Actor%20Object%20Reference) (OtherComp :type Primitive%20Component%20Object%20Reference) (OtherBodyIndex :type Integer) (bFromSweep :type Boolean) (SweepResult :type Hit%20Result%20Structure%20%28by%20ref%29))
  ;[1 1 1] Player checks if they've landed on an object they can bounce from
  (if (and (Utilities|DoesObjectImplementInterface OtherActor "/Game/Blueprints/Interfaces/BPI_PlayerBounceInterface.BPI_PlayerBounceInterface_C") (AI|Components|NavMovement|IsFalling (Variables|Character|GetCharacterMovement)))
    ;;[1 1 1] If the interface method Get Is Spring returns false, player is bouncing off of an enemy. If it returns true, the player is bouncing off of a spring
    (Class|BPIPlayerBounceInterface|GetIsSpring(Message) OtherActor)
    (if false
      (Character|LaunchCharacter "0.000000,0.000000,100.000000" false false)
      ;;;[1 0.2885 0.3061] Use the launch character to make it bounce, avoid use the speed setting
      (Audio|PlaySound2D "/Game/Sounds/Bounce_1.Bounce_1" 1.0 1.0 0.0 0 0)
      (else
        (Class|BPIPlayerBounceInterface|PlayerBouncedonEnemy(Message) OtherActor)
        (Character|LaunchCharacter "0.000000,0.000000,400.000000" false true)
        (Audio|PlaySound2D "/Game/Sounds/Bounce_1.Bounce_1" 1.0 1.0 0.0 0 0)))))

(event Custom|PushingBox
  (Variables|Default|SetIsPushingBox true)
  (Class|PaperZDAnimInstance|JumptoNode (Variables|/Script/PaperZD.PaperZDAnimationComponent|GetAnimInstance (Variables|Default|GetAnimationComponent)) "Pushing" "None"))

(event Input|EnhancedActionEvents|EnhancedInputActionIA_Move
  (params (ActionValue :type Float%20%28double-precision%29) (ElapsedSeconds :type Float%20%28double-precision%29) (TriggeredSeconds :type Float%20%28double-precision%29) (InputAction :type Input%20Action%20Object%20Reference :default "/Game/Blueprints/Core/Inputs/InputActions/IA_Move.IA_Move"))
  (if (not (or (Utilities|Enum|Equal(Enum) (Variables|Default|GetPlayerSM) "NewEnumerator3") (Utilities|Enum|Equal(Enum) (Variables|Default|GetPlayerSM) "NewEnumerator4")))
    (bind _output_get (Variables|Default|SetLastInputMovement ActionValue)) ; Variable for the  face direction in ABP instance
    (Pawn|Input|AddMovementInput "1.000000,0.000000,0.000000" _output_get false)))

(event Input|EnhancedActionEvents|EnhancedInputActionAI_Pause
  (params (ActionValue :type Boolean) (ElapsedSeconds :type Float%20%28double-precision%29) (TriggeredSeconds :type Float%20%28double-precision%29) (InputAction :type Input%20Action%20Object%20Reference :default "/Game/Blueprints/Core/Inputs/InputActions/AI_Pause.AI_Pause"))
  ;[0.02708 0.02708 0.02708] Call the pause widget BP to pause the game and show the pause menu
  (:Started
    (bind _ashud_in_game (Utilities|Casting|CastToHUD_InGame (HUD|GetHUD (Game|GetPlayerController 0)))
      (:then
        (Default|TogglePauseMenu (Variables|/Game/UI/GameplayMenu/W_GameInterface.W_GameInterface_C|GetW_PauseMenu (Variables|/Game/UI/GameplayMenu/HUD_InGame.HUD_InGame_C|GetW_GameInterface _ashud_in_game))))
      (:CastFailed
        (Development|PrintString "The hud class is null")))))

(event EventBeginPlay
  (|CallParentFunction))

(event EventOnLanded
  (params (Hit :type Hit%20Result%20Structure%20%28by%20ref%29))
  (Audio|PlaySound2D "/Game/Sounds/PlayerSounds/Landing_softlyCue.Landing_softlyCue" 1.0 1.0 0.0 0 0)
  (Components|Activation|Deactivate (Variables|Default|GetWindSoundEffect))
  (Audio|Components|Audio|FadeOut (Variables|Default|GetWindSoundEffect) 0.5 0.0 "Linear" :!class /Script/Engine.AudioComponent)
  (Utilities|FlowControl|RetriggerableDelay 0.5)
  (if (AI|Components|NavMovement|IsMovingonGround (Variables|Character|GetCharacterMovement))
    (Audio|Components|Audio|Stop (Variables|Default|GetWindSoundEffect))
    (Variables|Default|SetIsOnAir false)))

(event EventDamagePlayer
  (CallFunction|PlayerDying)
  (Components|Activation|Deactivate (Variables|Default|GetWindSoundEffect))
  (Audio|Components|Audio|Stop (Variables|Default|GetWindSoundEffect))
  (Variables|Default|SetIsOnAir false)
  (Audio|PlaySound2D "/Game/Sounds/PlayerSounds/Taking_damage_2_Cue.Taking_damage_2_Cue" 1.0 1.0 0.0 0 0)
  (Utilities|FlowControl|Delay 1.2)
  (Default|CallOnPlayerDeath)
  (CallFunction|PlayerRespawn))

(event EventOnWalkingOffLedge
  (params (PreviousFloorImpactNormal :type Vector%20%28by%20ref%29 :default "0, 0, 0") (PreviousFloorContactNormal :type Vector%20%28by%20ref%29 :default "0, 0, 0") (PreviousLocation :type Vector%20%28by%20ref%29 :default "0, 0, 0") (TimeDelta :type Float%20%28single-precision%29))
  (bind _windsoundeffect (Variables|Default|GetWindSoundEffect))
  ;[0.01562 0.01562 0.01562] Send a message to the ABP to play the fall animation when character falls
  (Class|PaperZDAnimInstance|JumptoNode (Variables|/Script/PaperZD.PaperZDAnimationComponent|GetAnimInstance (Variables|Default|GetAnimationComponent)) "Airbone" "None")
  (Components|Activation|Activate _windsoundeffect false)
  (Utilities|FlowControl|RetriggerableDelay 0.4)
  (if (Components|Activation|IsActive _windsoundeffect)
    (Audio|Components|Audio|Play (Variables|Default|GetWindSoundEffect) 0.0)
    (Variables|Default|SetIsOnAir true)))

(event EventMushroomBounce
  (bind _returnvalue (Transformation|GetVelocity))
  (if (< (.z _returnvalue) 0.0)
    (Character|LaunchCharacter (Math|Vector|MakeVector (.x _returnvalue) (.y _returnvalue) (* (.z _returnvalue) -1.8)) true true)))

(event EventOnJumped
  (bind _windsoundeffect (Variables|Default|GetWindSoundEffect))
  ;[0.01562 0.01562 0.01562] Send a message to the ABP to play the fall animation when character falls
  (Class|PaperZDAnimInstance|JumptoNode (Variables|/Script/PaperZD.PaperZDAnimationComponent|GetAnimInstance (Variables|Default|GetAnimationComponent)) "Airbone" "None")
  (Components|Activation|Activate _windsoundeffect false)
  (Utilities|FlowControl|RetriggerableDelay 0.4)
  (if (Components|Activation|IsActive _windsoundeffect)
    (Audio|Components|Audio|Play (Variables|Default|GetWindSoundEffect) 0.0)
    (Variables|Default|SetIsOnAir true)))

(event EventOnLaunched
  (params (LaunchVelocity :type Vector :default "0, 0, 0") (bXYOverride :type Boolean) (bZOverride :type Boolean))
  ;[0.03229 0.03229 0.03229] Send a message to the ABP to play the launch animation when character is launch
  (Class|PaperZDAnimInstance|JumptoNode (Variables|/Script/PaperZD.PaperZDAnimationComponent|GetAnimInstance (Variables|Default|GetAnimationComponent)) "Launch" "None"))

(event Input|KeyboardEvents|DebugKeyK
  (params (Key :type Key%20Structure :default "None") (ActionValue :type Input%20Action%20Value%20Structure))
  ;[0.4021 0.1751 0.1751] This action tests what will happen when the player reaches the goal (for testing only)
  (:Pressed
    (bind _ashud_in_game (Utilities|Casting|CastToHUD_InGame (HUD|GetHUD (Game|GetPlayerController 0))))
    (Default|CEndLevelMenu (Variables|/Game/UI/GameplayMenu/HUD_InGame.HUD_InGame_C|GetW_GameInterface _ashud_in_game))))

(fn ConstructionScript
  (|CallParentFunction))

(fn PlayerDying
  (bind _charactermovement (Variables|Character|GetCharacterMovement))
  (Components|Movement|StopMovementImmediately _charactermovement)
  (Variables|/Script/Engine.CharacterMovementComponent|SetGravityScale _charactermovement 0.0)
  (Variables|Default|SetPlayerSM "NewEnumerator3"))

(fn PlayerRespawn
  (Variables|/Script/Engine.CharacterMovementComponent|SetGravityScale (Variables|Character|GetCharacterMovement) 1.5)
  (Variables|Default|SetPlayerSM "NewEnumerator0")
  (Class|PaperZDAnimInstance|JumptoNode (Variables|/Script/PaperZD.PaperZDAnimationComponent|GetAnimInstance (Variables|Default|GetAnimationComponent)) "Respawn" "None"))