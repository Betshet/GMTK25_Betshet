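; BP_PuzzleBox is a physics-driven Paper2D puzzle box that the player can push and that falls.
; Each tick it moves the actor to its sprite's location and, while falling, limits vertical velocity to a capped downward speed until it reaches zero.
; Box overlaps, ignoring BP_ScreenWrap, halt the box on begin and start falling on end.
; A separate PlayerCollision overlap toggles the player's pushing state.
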(event OnComponentBeginOverlap(PlayerCollision)
  (params (OverlappedComponent :type Primitive%20Component%20Object%20Reference) (OtherActor :type Actor%20Object%20Reference) (OtherComp :type Primitive%20Component%20Object%20Reference) (OtherBodyIndex :type Integer) (bFromSweep :type Boolean) (SweepResult :type Hit%20Result%20Structure%20%28by%20ref%29))
  (bind _asbp_player_character (Utilities|Casting|CastToBP_PlayerCharacter OtherActor))
  (Default|PushingBox _asbp_player_character))

(event OnComponentEndOverlap(PlayerCollision)
  (params (OverlappedComponent :type Primitive%20Component%20Object%20Reference) (OtherActor :type Actor%20Object%20Reference) (OtherComp :type Primitive%20Component%20Object%20Reference) (OtherBodyIndex :type Integer))
  (bind _asbp_player_character (Utilities|Casting|CastToBP_PlayerCharacter OtherActor))
  (Variables|/Game/Blueprints/Character/PlayerCharacter/BP_PlayerCharacter.BP_PlayerCharacter_C|SetIsPushingBox _asbp_player_character false))

(event OnComponentEndOverlap(Box)
  (params (OverlappedComponent :type Primitive%20Component%20Object%20Reference) (OtherActor :type Actor%20Object%20Reference) (OtherComp :type Primitive%20Component%20Object%20Reference) (OtherBodyIndex :type Integer))
  (Utilities|Casting|CastToBP_ScreenWrap OtherActor
    (:CastFailed
      (bind _returnvalue (Physics|GetPhysicsLinearVelocity (Variables|Default|GetPaperSprite) "None"))
      (Physics|SetPhysicsLinearVelocity (Variables|Default|GetPaperSprite) (Math|Vector|MakeVector 0.0 0.0 (.z _returnvalue)) false "None")
      (Variables|Default|SetFalling true))))

(event OnComponentBeginOverlap(Box)
  (params (OverlappedComponent :type Primitive%20Component%20Object%20Reference) (OtherActor :type Actor%20Object%20Reference) (OtherComp :type Primitive%20Component%20Object%20Reference) (OtherBodyIndex :type Integer) (bFromSweep :type Boolean) (SweepResult :type Hit%20Result%20Structure%20%28by%20ref%29))
  (Utilities|Casting|CastToBP_ScreenWrap OtherActor
    (:CastFailed
      (Physics|SetPhysicsLinearVelocity (Variables|Default|GetPaperSprite) "0, 0, 0" false "None")
      (Variables|Default|SetFalling false))))

(event EventTick
  (params (DeltaSeconds :type Float%20%28single-precision%29))
  (Utilities|FlowControl|Sequence
    (:then_0
      (Transformation|SetActorLocation (Transformation|GetWorldLocation (Variables|Default|GetPaperSprite)) false false))
    (:then_1
      (if (Variables|Default|GetFalling)
        (bind _returnvalue (Physics|GetPhysicsLinearVelocity (Variables|Default|GetPaperSprite) "None"))
        (Physics|SetPhysicsLinearVelocity (Variables|Default|GetPaperSprite) (Math|Vector|MakeVector 0.0 0.0 (Math|Float|Clamp(Float) (.z _returnvalue) -4e+02 0.0)) false "None")
        (if (== (.z _returnvalue) 0.0)
          (Variables|Default|SetFalling false))))))

(fn ConstructionScript)