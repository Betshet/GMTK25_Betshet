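; Player controller that sets up input and a custom camera when play begins.
; On BeginPlay it adds the default Enhanced Input mapping context and switches to game-only input with the mouse cursor hidden.
; It then spawns a BP_CustomCamera at the player pawn's location, passes the pawn as its reference, stores it and makes it the view target.
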(event EventBeginPlay
  (bind _returnvalue (Game|Player|GetPlayerPawn 0))
  (bind _returnvalue_2 (PlayerController|LocalPlayerSubsystems|GetEnhancedInputLocalPlayerSubsystem))
  (Utilities|FlowControl|Sequence
    (:then_0
      (Utilities|IsValid _returnvalue_2
        (:Is%20Valid
          (Input|AddMappingContext _returnvalue_2 "/Game/Blueprints/Core/Inputs/IMC_Default.IMC_Default" 0 "(bIgnoreAllPressedKeysUntilRelease=True,bForceImmediately=False,bNotifyUserSettings=False)"))))
    (:then_1
      (Input|SetInputModeGameOnly self false)
      (Variables|Default|SetbShowMouseCursor false))
    (:then_2
      (bind _returnvalue_3 (Game|SpawnActorfromClass "/Game/Blueprints/Character/PlayerCharacter/BP_CustomCamera.BP_CustomCamera_C" (Math|Transform|MakeTransform (Transformation|GetActorLocation _returnvalue) "0, 0, 0" "1.000000,1.000000,1.000000") "Undefined" "MultiplyWithRoot" 0 _returnvalue _returnvalue))
      (bind _output_get (Variables|Default|SetPlayerCamera _returnvalue_3))
      (Game|Player|SetViewTargetwithBlend _output_get 0.0 "VTBlend_Linear" 0.0 false))))

(fn ConstructionScript)