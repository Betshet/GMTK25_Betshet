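; BP_SmallObstacle is a small level obstacle that renders with a Paper2D tilemap.
; On BeginPlay it runs the parent logic, then randomly assigns one of two configured tilemaps to its tilemap component.
; It then resizes its Box component to that tilemap's bounds, so the box extent follows the chosen variant.
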(event EventBeginPlay
  (|CallParentFunction)
  (Class|PaperTileMapComponent|SetTileMap (Variables|Default|GetPaperTileMap) (select (Math|Random|RandomBool) (Variables|Default|GetTilemapToUse2) (Variables|Default|GetTilemapToUse1)))
  (Components|Box|SetBoxExtent (Variables|Default|GetBox) (.BoxExtent (Collision|GetComponentBounds (Variables|Default|GetPaperTileMap))) true))

(event Collision|EventActorBeginOverlap
  (params (OtherActor :type Actor%20Object%20Reference))
  (|CallParentFunction OtherActor) ; This node is disabled and will not be called.\nDrag off pins to build functionality.
)

(event EventTick
  (params (DeltaSeconds :type Float%20%28single-precision%29))
  (|CallParentFunction DeltaSeconds) ; This node is disabled and will not be called.\nDrag off pins to build functionality.
)

(fn ConstructionScript
  (|CallParentFunction))